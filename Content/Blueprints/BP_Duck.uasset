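; BP_Duck is a duck target that travels along a spline and awards a point when hit.
; After a BeginPlay delay, a timeline scaled by FullMovementTime moves the actor along the MovementLine spline from start to end.
; A hit on the Line001 mesh increments Points and calls PointUp on BP_GameModeBase, then destroys the duck.
; The construction script sets the mesh from ObjectMesh.
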(event OnComponentHit(Line001)
  (params (HitComponent :type Primitive%20Component%20Object%20Reference) (OtherActor :type Actor%20Object%20Reference) (OtherComp :type Primitive%20Component%20Object%20Reference) (NormalImpulse :type Vector :default "0, 0, 0") (Hit :type Hit%20Result%20Structure%20%28by%20ref%29))
  (bind _asbp_game_mode_base (Utilities|Casting|CastToBP_GameModeBase (Game|GetGameMode)))
  (Default|PointUp _asbp_game_mode_base)
  (Variables|/Game/Blueprints/BP_GameModeBase.BP_GameModeBase_C|SetPoints _asbp_game_mode_base (+ (Variables|/Game/Blueprints/BP_GameModeBase.BP_GameModeBase_C|GetPoints _asbp_game_mode_base) 1))
  (Actor|DestroyActor))

(event Custom|Duck_Move
  (bind _movement_line (Variables|Default|GetMovement_Line))
  (bind _spline (Variables|/Game/Blueprints/BP_Duck_Path.BP_Duck_Path_C|GetSpline _movement_line))
  (Components|Timeline|SetPlayRate (Variables|Default|GetDuck_Movement_Timeline) (/ 1.0 (Variables|Default|GetFull_Movement_Time)))
  (bind _move_track (Timeline|Duck_Movement_Timeline Play)
    (:Update
      (Transformation|SetActorLocation (Spline|GetLocationatDistanceAlongSpline _spline (Math|Float|Lerp 0.0 (Spline|GetSplineLength _spline) _move_track) "World") false false))))

(event EventBeginPlay
  (Utilities|FlowControl|Delay (Variables|Default|GetDuration))
  (CallFunction|DuckMove))

(fn ConstructionScript
  (Components|StaticMesh|SetStaticMesh (Variables|Default|GetLine001) (Variables|Default|GetObject%20Mesh)))