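; BP_Spike is a short-lived spike actor that scores a point when it hits something.
; On BeginPlay it sets a five-second lifespan and rotates its Cone component into orientation.
; Any Cone hit, with no check on the other actor, calls PointUp on BP_GameModeBase, then increments Points and destroys the spike.
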(event OnComponentHit(Cone)
  (params (HitComponent :type Primitive%20Component%20Object%20Reference) (OtherActor :type Actor%20Object%20Reference) (OtherComp :type Primitive%20Component%20Object%20Reference) (NormalImpulse :type Vector :default "0, 0, 0") (Hit :type Hit%20Result%20Structure%20%28by%20ref%29))
  (bind _asbp_game_mode_base (Utilities|Casting|CastToBP_GameModeBase (Game|GetGameMode)))
  (Default|PointUp _asbp_game_mode_base)
  (Variables|/Game/Blueprints/BP_GameModeBase.BP_GameModeBase_C|SetPoints _asbp_game_mode_base (+ (Variables|/Game/Blueprints/BP_GameModeBase.BP_GameModeBase_C|GetPoints _asbp_game_mode_base) 1))
  (Actor|DestroyActor))

(event EventBeginPlay
  (Actor|SetLifeSpan 5.0)
  (Transformation|AddRelativeRotation (Variables|Default|GetCone) "0.000000,90.000000,-90.000000" false false))

(fn ConstructionScript)